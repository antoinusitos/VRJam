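; A projectile actor that flies in a straight line and destroys itself two seconds after spawning.
; Move stores the passed velocity scaled by Speed, and Tick adds that velocity to the actor location each frame.
; Movement is not scaled by delta time and uses no sweep, so speed depends on frame rate and the move itself detects no blocking hits.
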(event Custom|Move
  (params (velocity :type Vector))
  (Variables|Default|Setvelocity (* velocity (Variables|Default|Getspeed))))

(event EventBeginPlay
  (Utilities|FlowControl|Delay 2.0)
  (Actor|DestroyActor))

(event EventTick
  (params (DeltaSeconds :type Float%20%28single-precision%29))
  (Transformation|SetActorLocation (+ (Transformation|GetActorLocation) (Variables|Default|Getvelocity)) false false))

(fn ConstructionScript)