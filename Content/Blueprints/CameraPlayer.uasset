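; Player camera Blueprint that steers a separate character, the first ACharacter found at BeginPlay, through move, dodge, attack and fire inputs.
; Each tick a camera-forward trace places a decal and the ImpactPoint that aims every action.
; Holding Move pathfinds toward that point within range; dodge launches toward it, with timed cooldowns on dodge and attack.
; Server events mirror state and actions, while movement, attack and projectile spawning also run locally.
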(event Custom|Server_Dodge
  (params (rot :type Rotator) (velocity :type Vector))
  (bind _character (Variables|Default|Getcharacter))
  ;[1 1 1] dodge
  (Transformation|SetActorRotation _character rot)
  (Character|LaunchCharacter _character velocity false false)
  (Default|Dodge _character (Variables|Default|GetdodgeCost)))

(event Custom|Server_MoveToLocation
  (params (location :type Vector) (controller :type Controller%20Object%20Reference))
  ;[1 1 1] move to location
  (AI|Navigation|SimpleMovetoLocation controller location))

(event Custom|Server_Move
  (params (move :type Boolean))
  ;[1 1 1] check move
  (Variables|Default|SetmustMove move))

(event Custom|Server_SetImpactPoint
  (params (impact :type Vector))
  ;[1 1 1] set target
  (Variables|Default|SetImpactPoint impact))

(event Custom|Fire
  (bind _impactpoint (Variables|Default|GetImpactPoint))
  (bind _character (Variables|Default|Getcharacter))
  (bind _returnvalue (Transformation|GetActorLocation _character))
  (bind _returnvalue_2 (- _impactpoint _returnvalue))
  (bind (_x _y) (Math|Vector|BreakVector _returnvalue_2))
  ;[1 1 1] fire
  (bind _returnvalue_3 (Game|SpawnActorfromClass "/Game/Blueprints/Projectile.Projectile_C" (Math|Conversions|ToTransform(Vector) (Transformation|GetActorLocation (Variables|Default|Getcharacter))) "Undefined" 0 0))
  (Default|Move _returnvalue_3 (Math|Vector|Normalize (Math|Vector|MakeVector _x _y 0.0))))

(event Custom|Attack
  ;[1 1 1] attack
  (Default|GiveDamage (Variables|Default|Getcharacter) (Variables|Default|GetImpactPoint))
  (Utilities|FlowControl|Delay (Variables|Default|GettimeToAttack))
  (Variables|Default|SetcanAttack true))

(event Custom|Dodge
  (params (rot :type Rotator) (vel :type Vector))
  (bind _character (Variables|Default|Getcharacter))
  ;[1 1 1] dodge
  (Transformation|SetActorRotation _character rot)
  (Character|LaunchCharacter _character vel false false)
  (Default|Dodge _character (Variables|Default|GetdodgeCost)))

(event Custom|Server_Fire
  (bind _impactpoint (Variables|Default|GetImpactPoint))
  (bind _character (Variables|Default|Getcharacter))
  (bind _returnvalue (Transformation|GetActorLocation _character))
  (bind _returnvalue_2 (- _impactpoint _returnvalue))
  (bind (_x _y) (Math|Vector|BreakVector _returnvalue_2))
  ;[1 1 1] fire
  (bind _returnvalue_3 (Game|SpawnActorfromClass "/Game/Blueprints/Projectile.Projectile_C" (Math|Conversions|ToTransform(Vector) (Transformation|GetActorLocation (Variables|Default|Getcharacter))) "Undefined" 0 0))
  (Default|Move _returnvalue_3 (Math|Vector|Normalize (Math|Vector|MakeVector _x _y 0.0))))

(event Custom|Server_Attack
  ;[1 1 1] attack
  (Default|GiveDamage (Variables|Default|Getcharacter) (Variables|Default|GetImpactPoint))
  (Utilities|FlowControl|Delay (Variables|Default|GettimeToAttack))
  (Variables|Default|SetcanAttack true))

(event EventBeginPlay
  ;[1 1 1] begin play
  (bind _outactors (Actor|GetAllActorsOfClass "/Game/Blueprints/ACharacter.ACharacter_C"))
  (Variables|Default|Setcharacter (Utilities|Array|Get(acopy) _outactors))
  (Variables|Default|SettimeToAttack 1.0)
  (Variables|Default|SetcanAttack true)
  (Variables|Default|SetdistToMove 1e+03)
  (Variables|Default|SettimetoDodge 2.0)
  (Variables|Default|SetcanDodge true)
  (Variables|Default|SetdodgeForce 3e+03)
  (Variables|Default|SetdodgeCost 2e+01))

(event EventTick
  (params (DeltaSeconds :type Float%20%28single-precision%29))
  (bind _camera (Variables|Default|GetCamera))
  (bind _character (Variables|Default|Getcharacter))
  (bind _character_2 (Variables|Default|Getcharacter))
  (bind _returnvalue (Pawn|GetController _character_2))
  (bind _returnvalue_2 (Transformation|GetWorldLocation _camera))
  (Utilities|FlowControl|Sequence
    (:then_0
      ;[1 1 1] set target
      (bind (_outhit _returnvalue_3) (Collision|LineTraceByChannel _returnvalue_2 (+ _returnvalue_2 (* (Math|Vector|GetForwardVector _camera) 5e+03)) "TraceTypeQuery1" false 0 "None"))
      (if _returnvalue_3
        (Transformation|SetWorldLocation (Variables|Default|GetDecal) (.ImpactPoint (Collision|BreakHitResult _outhit)) false false)
        (bind _output_get (Variables|Default|SetImpactPoint (.ImpactPoint (Collision|BreakHitResult _outhit))))
        (CallFunction|ServerSetImpactPoint _output_get)))
    (:then_1
      ;[1 1 1] move to location
      (if (Variables|Default|GetmustMove)
        (if (<= (Math|Vector|VectorLength (- (Transformation|GetActorLocation _character_2) (Variables|Default|GetImpactPoint))) (Variables|Default|GetdistToMove))
          (CallFunction|ServerMovetoLocation (Variables|Default|GetImpactPoint) _returnvalue)
          (AI|Navigation|SimpleMovetoLocation _returnvalue (Variables|Default|GetImpactPoint)))))
    (:then_2
      ;[1 1 1] rotateUI
      (Utilities|IsValid _character
        (:Is%20Valid
          (Default|SetTextRotation _character (Transformation|GetActorLocation)))))))

(event Input|ActionEvents|InputActionMove
  (params (Key :type Key%20Structure :default "AnyKey"))
  ;[1 1 1] check move
  (:Pressed
    (bind _output_get (Variables|Default|SetmustMove true))
    (CallFunction|ServerMove _output_get))
  (:Released
    (bind _output_get_2 (Variables|Default|SetmustMove false))
    (CallFunction|ServerMove _output_get_2)))

(event Input|ActionEvents|InputActionAttack
  (params (Key :type Key%20Structure :default "AnyKey"))
  ;[1 1 1] attack
  (:Pressed
    (if (Variables|Default|GetcanAttack)
      (Variables|Default|SetcanAttack false)
      (CallFunction|Attack)
      (CallFunction|ServerAttack))))

(event Input|ActionEvents|InputActionDodge
  (params (Key :type Key%20Structure :default "AnyKey"))
  (bind _character (Variables|Default|Getcharacter))
  (bind _impactpoint (Variables|Default|GetImpactPoint))
  (bind _returnvalue (Transformation|GetActorLocation _character))
  (bind _returnvalue_2 (- _impactpoint _returnvalue))
  (bind (_x _y) (Math|Vector|BreakVector _returnvalue_2))
  (bind _returnvalue_3 (Math|Vector|MakeVector _x _y 0.0))
  ;[1 1 1] dodge
  (:Pressed
    (if (Variables|Default|GetcanDodge)
      (Variables|Default|SetcanDodge false)
      (CallFunction|ServerDodge (Math|Rotator|MakeRotator 0.0 0.0 (.Yaw (Math|Rotator|BreakRotator (Math|Rotator|FindLookatRotation (Transformation|GetActorLocation _character) _returnvalue_3)))) (* (Math|Vector|Normalize _returnvalue_3) (Variables|Default|GetdodgeForce)))
      (Utilities|FlowControl|Delay (Variables|Default|GettimetoDodge))
      (Variables|Default|SetcanDodge true))))

(event Input|ActionEvents|InputActionFire
  (params (Key :type Key%20Structure :default "AnyKey"))
  ;[1 1 1] fire
  (:Pressed
    (CallFunction|Fire)
    (CallFunction|ServerFire)))

(fn ConstructionScript)