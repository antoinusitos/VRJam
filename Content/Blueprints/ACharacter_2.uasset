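; Player character Blueprint with health and mana, melee attack, mana-costing dodge and world-space stat bars.
; Attacking yaws toward the cursor and damages enemies overlapping AttackSphere; taking lethal damage only prints a loss message.
; Tick triggers server regeneration of both stats, which multicasts to update the bars.
; Bars turn toward a supplied camera location and multiply their current Y scale by the stat ratio, so scaling compounds.
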(event Custom|SetTextRotation
  (params (locationCam :type Vector))
  (bind _health (Variables|Default|GetHealth))
  (bind _mana (Variables|Default|GetMana))
  ;[1 1 1] set ui rotation
  (Transformation|SetWorldRotation _health (Math|Rotator|FindLookatRotation (Transformation|GetWorldLocation _health) locationCam) false false)
  (Transformation|SetWorldRotation _mana (Math|Rotator|FindLookatRotation (Transformation|GetWorldLocation _mana) locationCam) false false))

(event Custom|GiveDamage
  (params (cursorLocation :type Vector))
  ;[1 1 1] give damage
  (Transformation|SetActorRotation (Math|Rotator|MakeRotator 0.0 0.0 (.Yaw (Math|Rotator|BreakRotator (Math|Rotator|FindLookatRotation (Transformation|GetActorLocation) cursorLocation)))))
  (for _array_element (Collision|GetOverlappingActors (Variables|Default|GetattackSphere) "/Game/Blueprints/enemy.enemy_C" :!class /Script/Engine.PrimitiveComponent)
    (bind _asenemy (Utilities|Casting|CastToenemy _array_element))
    (Default|TakeDamage _asenemy (Variables|Default|Getdamage))))

(event Custom|Multicast_Refill
  (params (life :type Float%20%28single-precision%29) (mana :type Float%20%28single-precision%29))
  (bind _health (Variables|Default|GetHealth))
  (bind _mana (Variables|Default|GetMana))
  (bind _relativescale3d (Variables|/Script/Engine.SceneComponent|GetRelativeScale3D _mana))
  (bind _relativescale3d_2 (Variables|/Script/Engine.SceneComponent|GetRelativeScale3D _health))
  (bind (_x _y _z) (Math|Vector|BreakVector _relativescale3d))
  (bind (_x_2 _y_2 _z_2) (Math|Vector|BreakVector _relativescale3d_2))
  ;[1 1 1] refill mana and life
  (Transformation|SetRelativeScale3D _mana (Math|Vector|MakeVector _x (* _y (/ mana (Variables|Default|GetmaxMana))) _z))
  (Transformation|SetRelativeScale3D _health (Math|Vector|MakeVector _x_2 (* _y_2 (/ life (Variables|Default|GetmaxLife))) _z_2))
  (Development|PrintString (Utilities|String|ToString(Float) (Variables|Default|GetcurrentMana)) true true "(R=0.000000,G=0.660000,B=1.000000,A=1.000000)" 0.0))

(event Custom|Dodge
  (params (amount :type Float%20%28single-precision%29))
  (bind _mana (Variables|Default|GetMana))
  (bind _relativescale3d (Variables|/Script/Engine.SceneComponent|GetRelativeScale3D _mana))
  (bind (_x _y _z) (Math|Vector|BreakVector _relativescale3d))
  ;[1 1 1] empty mana for dodge
  (Variables|Default|SetcurrentMana (- (Variables|Default|GetcurrentMana) amount))
  (Transformation|SetRelativeScale3D _mana (Math|Vector|MakeVector _x (* _y (/ (Variables|Default|GetcurrentMana) (Variables|Default|GetmaxMana))) _z)))

(event Custom|Server_refill
  (bind _returnvalue (Utilities|Time|GetWorldDeltaSeconds))
  ;[1 1 1] refill mana and life
  (bind _output_get (Variables|Default|Setlife (+ (Variables|Default|Getlife) _returnvalue)))
  (if (>= _output_get (Variables|Default|GetmaxLife))
    (Variables|Default|Setlife (Variables|Default|GetmaxLife)))
  (bind _output_get_2 (Variables|Default|SetcurrentMana (+ (Variables|Default|GetcurrentMana) _returnvalue)))
  (if (>= _output_get_2 (Variables|Default|GetmaxMana))
    (Variables|Default|SetcurrentMana (Variables|Default|GetmaxMana)))
  (CallFunction|MulticastRefill (Variables|Default|Getlife) (Variables|Default|GetcurrentMana)))

(event Custom|TakeDamage
  (params (amount :type Float%20%28single-precision%29))
  (bind _health (Variables|Default|GetHealth))
  (bind _relativescale3d (Variables|/Script/Engine.SceneComponent|GetRelativeScale3D _health))
  (bind (_x _y _z) (Math|Vector|BreakVector _relativescale3d))
  ;[1 1 1] take damage
  (bind _output_get (Variables|Default|Setlife (- (Variables|Default|Getlife) amount)))
  (Transformation|SetRelativeScale3D _health (Math|Vector|MakeVector _x (* _y (/ (Variables|Default|Getlife) (Variables|Default|GetmaxLife))) _z))
  (if (<= _output_get 0.0)
    (Development|PrintString "LOOSE")))

(event EventTick
  (params (DeltaSeconds :type Float%20%28single-precision%29))
  ;[1 1 1] refill mana and life
  (CallFunction|ServerRefill))

(event EventBeginPlay
  ;[1 1 1] begin play
  (Variables|Default|Setlife 1e+02)
  (Variables|Default|SetmaxLife 1e+02)
  (Transformation|SetRelativeScale3D (Variables|Default|GetHealth) (Math|Vector|MakeVector 0.05 0.5 0.05))
  (Variables|Default|Setdamage 5e+01)
  (bind _output_get (Variables|Default|SetmaxMana 1e+02))
  (Variables|Default|SetcurrentMana _output_get)
  (Transformation|SetRelativeScale3D (Variables|Default|GetMana) (Math|Vector|MakeVector 0.05 0.5 0.05)))

(fn ConstructionScript)