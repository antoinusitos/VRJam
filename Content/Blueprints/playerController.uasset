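; Player controller that spawns a character for the CameraPlayer pawn when Init runs on the server.
; Init spawns an ACharacter at the first SpawnPoint, assigns it to player 0's CameraPlayer rather than its own pawn, then destroys that spawn point.
; It also calls OwnerSetCharacter, whose matching event only prints a debug string.
; The CameraPlayer attack, movement and dodge setup is disconnected and never runs.
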(event Custom|Init
  (Networking|SwitchHasAuthority
    (:Authority
      (bind _outactors (Actor|GetAllActorsOfClass "/Game/Blueprints/SpawnPoint.SpawnPoint_C"))
      (bind _returnvalue (Game|SpawnActorfromClass "/Game/Blueprints/ACharacter.ACharacter_C" (Math|Conversions|ToTransform(Vector) (Transformation|GetActorLocation (Utilities|Array|Get(acopy) _outactors))) "Undefined" 0 0))
      (bind _ascamera_player (Utilities|Casting|CastToCameraPlayer (Game|Player|GetPlayerPawn 0)))
      (Variables|/Game/Blueprints/CameraPlayer.CameraPlayer_C|Setcharacter _ascamera_player _returnvalue)
      (CallFunction|OwnerSetCharacter _returnvalue)
      (Actor|DestroyActor (Utilities|Array|Get(acopy) _outactors)))))

(event Custom|Owner_SetCharacter
  (params (character :type A%20Character%20Object%20Reference))
  (Development|PrintString "Hello"))

(event EventBeginPlay)

(fn ConstructionScript)