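; Enemy actor that chases a character it detects and deals melee damage at close range.
; SeePlayer overlaps set or clear the target; Tick moves toward it or attacks, with a Delay as cooldown, and losing it halts movement.
; Projectiles entering DamageSphere apply their damage and are destroyed.
; Damage rescales the Health bar's current Y by remaining life fraction, so shrinkage compounds per hit; zero life destroys the enemy.
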(event OnComponentBeginOverlap(SeePlayer)
  (params (OtherActor :type Actor%20Object%20Reference) (OtherComp :type Primitive%20Component%20Object%20Reference) (OtherBodyIndex :type Integer) (bFromSweep :type Boolean) (SweepResult :type Hit%20Result%20Structure%20%28by%20ref%29))
  (bind _asacharacter (Utilities|Casting|CastToACharacter OtherActor))
  (Variables|Default|Setenemy _asacharacter))

(event OnComponentEndOverlap(SeePlayer)
  (params (OtherActor :type Actor%20Object%20Reference) (OtherComp :type Primitive%20Component%20Object%20Reference) (OtherBodyIndex :type Integer))
  (if (== OtherActor (Variables|Default|Getenemy))
    (Variables|Default|Setenemy 0)
    (AI|Navigation|SimpleMovetoLocation (Pawn|GetController) (Transformation|GetActorLocation))))

(event OnComponentBeginOverlap(damageSphere)
  (params (OtherActor :type Actor%20Object%20Reference) (OtherComp :type Primitive%20Component%20Object%20Reference) (OtherBodyIndex :type Integer) (bFromSweep :type Boolean) (SweepResult :type Hit%20Result%20Structure%20%28by%20ref%29))
  (bind _asprojectile (Utilities|Casting|CastToProjectile OtherActor))
  (CallFunction|TakeDamage (Variables|/Game/Blueprints/Projectile.Projectile_C|Getdamage _asprojectile))
  (Actor|DestroyActor _asprojectile))

(event Custom|TakeDamage
  (params (damage :type Float%20%28single-precision%29))
  (bind _health (Variables|Default|GetHealth))
  (bind _relativescale3d (Variables|/Script/Engine.SceneComponent|GetRelativeScale3D _health))
  (bind (_x _y _z) (Math|Vector|BreakVector _relativescale3d))
  (bind _output_get (Variables|Default|Setlife (- (Variables|Default|Getlife) damage)))
  (Transformation|SetRelativeScale3D _health (Math|Vector|MakeVector _x (* _y (/ (Variables|Default|Getlife) (Variables|Default|GetmaxLife))) _z))
  (if (<= _output_get 0.0)
    (Actor|DestroyActor)))

(event EventTick
  (params (DeltaSeconds :type Float%20%28single-precision%29))
  (if (Utilities|IsValid (Variables|Default|Getenemy))
    (if (<= (Transformation|GetDistanceTo (Variables|Default|Getenemy)) 1e+02)
      (if (Variables|Default|GetcanAttack)
        (Variables|Default|SetcanAttack false)
        (Default|TakeDamage (Variables|Default|Getenemy) (Variables|Default|Getdamage))
        (Utilities|FlowControl|Delay (Variables|Default|GettimeToAttack))
        (Variables|Default|SetcanAttack true))
      (else
        (AI|Navigation|SimpleMovetoActor (Pawn|GetController) (Variables|Default|Getenemy))))))

(event EventBeginPlay
  (Variables|Default|SetcanAttack true)
  (Variables|Default|SettimeToAttack 1.0)
  (bind _output_get (Variables|Default|SetmaxLife 1e+02))
  (Variables|Default|Setlife _output_get)
  (Variables|Default|Setdamage 1e+01)
  (Transformation|SetRelativeScale3D (Variables|Default|GetHealth) (Math|Vector|MakeVector 0.05 0.5 0.05)))

(fn ConstructionScript)